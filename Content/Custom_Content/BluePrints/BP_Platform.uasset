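; BP_Platform is a side-scroller platform that starts without collision and lights up green when the player character first lands on it.
; CollisonTrigger enables the mesh's collision on begin overlap and disables it on end overlap.
; An overlap with the platform itself permanently sets StuckCheck, blocking further enabling.
; The first character hit calls LandOnPlatform and recolors the point light and dynamic material created at construction.
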(event `self.Collison Trigger.OnComponentBeginOverlap`
  (params (OtherActor :type "Actor Object Reference") (OtherComp :type "PrimitiveComponent Object Reference") (OtherBodyIndex :type Integer) (bFromSweep :type Boolean) (SweepResult :type "HitResult Structure (by ref)"))
  (if (not (`self.Stuck Check`))
    (`PrimitiveComponent.SetCollisionEnabled` (`self.Me_Platform`) "QueryAndPhysics")))

(event `self.Me_Platform.OnComponentBeginOverlap`
  (params (OtherActor :type "Actor Object Reference") (OtherComp :type "PrimitiveComponent Object Reference") (OtherBodyIndex :type Integer) (bFromSweep :type Boolean) (SweepResult :type "HitResult Structure (by ref)"))
  (set `self.Stuck Check` true))

(event `self.Collison Trigger.OnComponentEndOverlap`
  (params (OtherActor :type "Actor Object Reference") (OtherComp :type "PrimitiveComponent Object Reference") (OtherBodyIndex :type Integer))
  (`PrimitiveComponent.SetCollisionEnabled` (`self.Me_Platform`) "NoCollision"))

(event `self.Me_Platform.OnComponentHit`
  (params (OtherActor :type "Actor Object Reference") (OtherComp :type "PrimitiveComponent Object Reference") (NormalImpulse :type "Vector Structure") (Hit :type "HitResult Structure (by ref)"))
  (if (not (`self.Hit!`))
    (bind _asside_scroller_character (cast `/Game/Custom_Content/BluePrints/SideScrollerCharacter` OtherActor))
    (`/Game/Custom_Content/BluePrints/SideScrollerCharacter.Land on Platform` _asside_scroller_character)
    (`MaterialInstanceDynamic.SetVectorParameterValue` (`self.Dynamic Material`) "Light" (struct :`G` 0.905 :`B` 0.086276 :`A` 1.0))
    (`LightComponent.SetLightColor` (`self.PointLight`) (struct :`G` 1.0 :`B` 0.076539 :`A` 1.0) true)
    (set `self.Hit!` true)))

(fn `UserConstructionScript`
  (`|ExecutionSequence`
    (:`then_0`
      (`PrimitiveComponent.SetCollisionEnabled` (`self.Me_Platform`) "NoCollision"))
    (:`then_1`
      (bind _returnvalue (`PrimitiveComponent.CreateDynamicMaterialInstance` (`self.Me_Platform`) 2 null))
      (set `self.Dynamic Material` _returnvalue))))