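; BP_Door is a side-scroller door that turns its lights green when the player character enters its trigger box.
; The construction script creates a dynamic material instance on the door mesh and disables the mesh's collision.
; On overlap, FinishColorChange sets the material's Door_Light parameter to green and recolors the six RedLight components to match.
; Nothing in the graph switches the lights back.
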(event `self.Box.OnComponentBeginOverlap`
  (params (OtherActor :type "Actor Object Reference") (OtherComp :type "PrimitiveComponent Object Reference") (OtherBodyIndex :type Integer) (bFromSweep :type Boolean) (SweepResult :type "HitResult Structure (by ref)"))
  (cast `/Game/Custom_Content/BluePrints/SideScrollerCharacter` OtherActor)
  (`self.Finish Color Change`))

(fn `Finish Color Change`
  (`|ExecutionSequence`
    (:`then_0`
      (`MaterialInstanceDynamic.SetVectorParameterValue` (`self.Dynamic Material`) "Door_Light" (struct :`R` 0.002509 :`G` 0.59 :`A` 1.0)))
    (:`then_1`
      (`LightComponent.SetLightColor` (`self.Red Light 1`) (struct :`G` 0.795 :`B` 0.038176 :`A` 1.0) true)
      (`LightComponent.SetLightColor` (`self.Red Light 2`) (struct :`G` 0.795 :`B` 0.038176 :`A` 1.0) true)
      (`LightComponent.SetLightColor` (`self.Red Light 3`) (struct :`G` 0.795 :`B` 0.038176 :`A` 1.0) true)
      (`LightComponent.SetLightColor` (`self.Red Light 4`) (struct :`G` 0.795 :`B` 0.038176 :`A` 1.0) true)
      (`LightComponent.SetLightColor` (`self.Red Light 5`) (struct :`G` 0.795 :`B` 0.038176 :`A` 1.0) true)
      (`LightComponent.SetLightColor` (`self.Red Light 6`) (struct :`G` 0.795 :`B` 0.038176 :`A` 1.0) true))))

(fn `UserConstructionScript`
  (`|ExecutionSequence`
    (:`then_0`
      (bind _returnvalue (`PrimitiveComponent.CreateDynamicMaterialInstance` (`self.Me_Door`) 2 null))
      (set `self.Dynamic Material` _returnvalue))
    (:`then_1`
      (`PrimitiveComponent.SetCollisionEnabled` (`self.Me_Door`) "NoCollision"))))